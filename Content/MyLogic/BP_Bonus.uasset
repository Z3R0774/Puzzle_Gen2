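; BP_Bonus is a bonus actor whose Cube moves each tick along Direct at Speed, using a swept offset.
; A life flag, set through the Alive? event, gates that movement; when false, the actor destroys itself on Tick.
; Deviltrigger clears the flag and sets Jackpot, so the destroy branch also calls J4ckpot, which prints a "Jackpot!" message.
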(event `self.ReceiveTick`
  (params (DeltaSeconds :type "Float (single-precision)"))
  (if (`self.LiFe Stat`)
    (`SceneComponent.K2_AddWorldOffset` (`self.Cube`) (* (* (`self.Direct`) (`self.Speed`)) DeltaSeconds) true false)
    (else
      (`self.K2_DestroyActor`)
      (if (`self.Jackpot`)
        (`self.J4ckpot`)))))

(event `/Game/MyLogic/BPI_KI11.Alive?`
  (params (LiFeStat :type Boolean))
  (set `self.LiFe Stat` LiFeStat))

(event `/Game/MyLogic/BPI_Bonus.Deviltrigger`
  (params (NewParam1 :type Boolean))
  (set `self.LiFe Stat` false)
  (set `self.Jackpot` true))

(fn `J4ckpot`
  (`KismetSystemLibrary.PrintString` "Jackpot!"))

(fn `UserConstructionScript`)