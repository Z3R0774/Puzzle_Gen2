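; Player paddle that slides sideways within the Granitsa limit, launches the ball and tracks three lives.
; Each tick it sends its Sphere location to actors tagged "New"; the Release input sends them the launch message.
; A New? event with true costs a life, then spawns and notifies a BP_Ball at the Sphere, or destroys the paddle at zero.
; Communication uses interface messages, including Deviltrigger on Box overlap.
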(event `self.ReceiveTick`
  (params (DeltaSeconds :type "Float (single-precision)"))
  (bind _outactors (`GameplayStatics.GetAllActorsWithTag` "New"))
  (message `/Game/MyLogic/BPI_KI11.Location` _outactors (`SceneComponent.K2_GetComponentLocation` (`self.Sphere`))))

(event `self.ReceiveBeginPlay`
  ;[1 1 1] Start
  (bind _output_get (set `self.LIfeCounter` 3))
  (set `self.LF` (`KismetTextLibrary.Conv_IntToText` _output_get))
  (`KismetSystemLibrary.PrintString` (`KismetStringLibrary.Conv_IntToString` _output_get) true true (struct :`R` 0.018111 :`G` 0.5125 :`A` 1.0) 5.0)
  (set `self.Tags` (`|MakeArray` (`self.Platform`)))
  (`self.EnableInput` (`GameplayStatics.GetPlayerController` 0))
  (`KismetSystemLibrary.PrintString` (`KismetTextLibrary.Conv_TextToString` (`self.LF`))))

(event `InputAxis|MoveRight`
  (params (AxisValue :type "Float (single-precision)"))
  (bind (_returnvalue_x _returnvalue_y) (`KismetMathLibrary.BreakVector` (`SceneComponent.K2_GetComponentLocation` (`self.Cube`))))
  ;[1 1 1] Movement
  (if (> _returnvalue_y (* (`self.Granitsa`) -1.0))
    (if (> AxisValue 0.0)
      (`SceneComponent.K2_AddWorldOffset` (`self.Cube`) (0.0 -50.0 0.0) false false))))

(event `InputAxis|MoveRight`
  (params (AxisValue :type "Float (single-precision)"))
  (bind (_returnvalue_x _returnvalue_y) (`KismetMathLibrary.BreakVector` (`SceneComponent.K2_GetComponentLocation` (`self.Cube`))))
  ;[1 1 1] Movement
  (if (< _returnvalue_y (`self.Granitsa`))
    (if (< AxisValue 0.0)
      (`SceneComponent.K2_AddWorldOffset` (`self.Cube`) (0.0 50.0 0.0) false false))))

(event `/Game/MyLogic/BPI_KI11.New?`
  (params (NewLife :type Boolean))
  (bind (_returnvalue_x _returnvalue_y _returnvalue_z) (`KismetMathLibrary.BreakVector` (`SceneComponent.K2_GetComponentLocation` (`self.Sphere`))))
  ;[1 1 1] Rojdenie
  (if NewLife
    (bind _output_get (set `self.LIfeCounter` (- (`self.LIfeCounter`) 1)))
    (set `self.LF` (`KismetTextLibrary.Conv_IntToText` _output_get))
    (`KismetSystemLibrary.PrintString` (`KismetStringLibrary.Conv_IntToString` _output_get) true true (struct :`R` 0.018111 :`G` 0.5125 :`A` 1.0) 5.0)
    (if (== (`self.LIfeCounter`) 0)
      (`self.K2_DestroyActor`)
      (`KismetSystemLibrary.PrintString` "Pres esc to try again" true true (struct :`R` 0.4 :`A` 1.0))
      (else
        (bind _returnvalue (`|SpawnActorFromClass` "/Game/MyLogic/BP_Ball.BP_Ball_C" (`KismetMathLibrary.MakeTransform` (`KismetMathLibrary.MakeVector` _returnvalue_x _returnvalue_y _returnvalue_z) (struct) (1.0 1.0 1.0)) "AlwaysSpawn" "OverrideRootScale" null null))
        (message `/Game/MyLogic/BPI_KI11.AnotherOne` _returnvalue "New")
        (bind _outactors (`GameplayStatics.GetAllActorsWithInterface` "/Game/MyLogic/BPI_KI11.BPI_KI11_C"))
        (message `/Game/MyLogic/BPI_KI11.New?` _outactors false)))))

(event `InputAction|Release`
  (params (Key :type "Key Structure"))
  ;[1 1 1] Launch ball
  (:`Pressed`
    (bind _output_get (set `self.Start?` true))
    (bind _outactors (`GameplayStatics.GetAllActorsWithTag` "New"))
    (message `/Game/MyLogic/BPI_KI11.Again?` _outactors _output_get)))

(event `self.Box.OnComponentBeginOverlap`
  (params (OverlappedComponent :type "PrimitiveComponent Object Reference") (OtherActor :type "Actor Object Reference") (OtherComp :type "PrimitiveComponent Object Reference") (OtherBodyIndex :type Integer) (bFromSweep :type Boolean) (SweepResult :type "HitResult Structure (by ref)"))
  (message `/Game/MyLogic/BPI_Bonus.Deviltrigger` OtherActor false))

(fn `LivesFunc`
  (params (NewParam1 :type Text))
  (returns (NewParam :type Text))
  (return ""))

(fn `Location`
  (params (Location :type "Vector Structure"))
  (return))

(fn `ScoreFunc`
  (params (ScIn :type Text))
  (returns (ScOut :type Text))
  (return ""))

(fn `UserConstructionScript`)