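; BP_Spawner is a spawner Blueprint whose J4ckpot function creates a BP_Ball in the level.
; It finds actors tagged "Platform" and spawns the ball at a fixed X offset from the first one's root location, then calls FirestarterMessage on the new ball.
; The event graph and construction script only forward to the parent, and nothing in this file calls J4ckpot.
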(event `self.ReceiveTick`
  (params (DeltaSeconds :type "Float (single-precision)"))
  (`parent.ReceiveTick` DeltaSeconds))

(fn `J4ckpot`
  (bind _outactors (`GameplayStatics.GetAllActorsWithTag` "Platform"))
  (bind _returnvalue (`|SpawnActorFromClass` "/Game/MyLogic/BP_Ball.BP_Ball_C" (`KismetMathLibrary.MakeTransform` (+ (`SceneComponent.K2_GetComponentLocation` (`Actor.RootComponent` (`|GetArrayItem` _outactors))) (-200.0 0.0 0.0))) "Undefined" "OverrideRootScale" null null))
  (message `/Game/MyLogic/BPI_KI11.Firestarter` _returnvalue "None"))

(fn `UserConstructionScript`
  (`parent.UserConstructionScript`))