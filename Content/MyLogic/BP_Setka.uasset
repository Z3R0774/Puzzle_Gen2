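; Block grid spawner (Setka) that builds a randomized field of BP_Block actors and tracks score and victory.
; On BeginPlay it spawns centered rows of random length, with a summon roll that always passes.
; Each spawn triggers a BPI_Points message to an indexed interface actor, giving about one in five bonus points.
; CountOfBlocks decrements the block count and shows WinScreen at zero, while Nachislenie accumulates score text.
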(event `self.ReceiveBeginPlay`
  (bind _space (`self.Space`))
  (set `self.center` (/ (* (`self.Gor`) (`self.Space`)) 2.0))
  (set `self.Tags` (`|MakeArray` (`self.Name`)))
  (for _index (range (`self.vert`))
    (bind _output_get (set `self.CurrentGor` (`KismetMathLibrary.RandomIntegerInRange` 1 (`self.Gor`))))
    (set `self.Delta` (- (`self.center`) (/ (* (`self.CurrentGor`) (`self.Space`)) 2.0)))
    (for _index_2 (range _output_get)
      (set `self.RandomNumberSummon` (`KismetMathLibrary.RandomIntegerInRange` 1 100))
      (set `self.RandomNumberSpecial` (`KismetMathLibrary.Conv_Int64ToInt` (`KismetMathLibrary.RandomInteger64InRange` 1 100)))
      (if (> (`self.RandomNumberSummon`) 0)
        (set `self.index` (+ (`self.index`) 1))
        (`|SpawnActorFromClass` "/Game/MyLogic/BP_Block.BP_Block_C" (`KismetMathLibrary.MakeTransform` (+ (`KismetMathLibrary.MakeVector` (/ (* _index _space) 2.0) (+ (`self.Delta`) (* _index_2 _space))) (`self.K2_GetActorLocation`)) (struct :`Yaw` 90.0) (`self.Scale`)) "Undefined" "OverrideRootScale" self null)
        (if (> (`self.RandomNumberSpecial`) 80)
          (set `self.Points` 3)
          (else
            (set `self.Points` 0)))
        (bind _outactors (`GameplayStatics.GetAllActorsWithInterface` "/Game/MyLogic/BPI_Points.BPI_Points_C"))
        (message `/Game/MyLogic/BPI_Points.Peredacha` (`|GetArrayItem` _outactors (`self.index`)) (`self.Points`) false)
        (set `self.Count` (+ (`self.Count`) 1))))))

(event `/Game/MyLogic/BPI_EndGame.CountOfBlocks`
  (params (`Destroyed?` :type Boolean))
  ;[1 1 1] End
  (bind _output_get (set `self.Count` (- (`self.Count`) 1)))
  (`KismetSystemLibrary.PrintString` (`KismetStringLibrary.Conv_IntToString` _output_get) true true (struct :`G` 0.013741 :`B` 1.0 :`A` 1.0))
  (if (== (`self.Count`) 0)
    (bind _returnvalue (`|CreateWidget` "/Game/MyLogic/WinScreen.WinScreen_C"))
    (`UserWidget.AddToViewport` _returnvalue 0)))

(event `/Game/MyLogic/BPI_Points.Nachislenie`
  (params (sc0re :type Integer))
  ;[1 1 1] Ochki
  (bind _output_get (set `self.Total score` (+ sc0re (`self.Total score`))))
  (set `self.TS` (`KismetTextLibrary.Conv_IntToText` _output_get)))

(fn `LivesFunc`
  (params (NewParam1 :type Text))
  (returns (NewParam :type Text))
  (return ""))

(fn `ScoreFunc`
  (params (ScIn :type Text))
  (returns (ScOut :type Text))
  (return ""))

(fn `UserConstructionScript`)