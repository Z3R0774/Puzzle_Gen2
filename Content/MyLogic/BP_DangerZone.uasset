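; BP_DangerZone is a trigger volume that reports a not-alive state to any actor entering its box.
; On BeginPlay it sets its tag and broadcasts an alive state to all BPI_KI11 implementers, then Box overlap sends false through AliveMessage.
; A BallCount event decrements a ball counter and prints a debug string, but nothing acts on the count.
; A message to Platform-tagged actors is left disconnected.
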(event `self.ReceiveBeginPlay`
  (set `self.BallC0unt` 1)
  (set `self.Tags` (`|MakeArray` (`self.NewVar_0`)))
  (bind _output_get (set `self.LiFeStat` true))
  (bind _outactors (`GameplayStatics.GetAllActorsWithInterface` "/Game/MyLogic/BPI_KI11.BPI_KI11_C"))
  (message `/Game/MyLogic/BPI_KI11.Alive?` _outactors _output_get))

(event `self.Box.OnComponentBeginOverlap`
  (params (OverlappedComponent :type "PrimitiveComponent Object Reference") (OtherActor :type "Actor Object Reference") (OtherComp :type "PrimitiveComponent Object Reference") (OtherBodyIndex :type Integer) (bFromSweep :type Boolean) (SweepResult :type "HitResult Structure (by ref)"))
  (bind _output_get (set `self.LiFeStat` false))
  (message `/Game/MyLogic/BPI_KI11.Alive?` OtherActor _output_get))

(event `/Game/MyLogic/BPI_KI11.BallCount`
  (params (NewParam :type Boolean))
  (set `self.Let's go` NewParam)
  (set `self.BallC0unt` (- (`self.BallC0unt`) 1))
  (`KismetSystemLibrary.PrintString` "Hello"))

(event `/Game/MyLogic/BPI_KI11.New?`
  (params (NewLife :type Boolean))
  (set `self.NewLife` NewLife))

(fn `UserConstructionScript`)