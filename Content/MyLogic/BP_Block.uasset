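; BP_Block is a hittable block that awards score when destroyed, with a special gold variant when Points equals 3.
; BeginPlay and Peredacha share logic that sets the gold material and a score of 500 for that variant, otherwise 100.
; Hit spawns BP_Spawner for gold blocks, destroys the Cube component, then messages "Setka"-tagged actors to update block count and score.
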(event `self.ReceiveBeginPlay`
  (set `self.Tags` (`self.Block`))
  (if (== 3 (stale `/Game/MyLogic/BPI_Points.Peredacha` Points)) :!label _label
    (`PrimitiveComponent.SetMaterial` (`self.Cube`) 0 "/Game/StarterContent/Materials/M_Metal_Gold.M_Metal_Gold")
    (set `self.sc0re` 500)
    (else
      (set `self.sc0re` 100))))

(event `/Game/MyLogic/BPI_Points.Peredacha`
  (params (Points :type Integer) (Visivility :type Boolean))
  (goto _label))

(event `self.ReceiveHit`
  (params (MyComp :type "PrimitiveComponent Object Reference") (Other :type "Actor Object Reference") (OtherComp :type "PrimitiveComponent Object Reference") (bSelfMoved :type Boolean) (HitLocation :type "Vector Structure") (HitNormal :type "Vector Structure") (NormalImpulse :type "Vector Structure") (Hit :type "HitResult Structure (by ref)"))
  (if (== (stale `/Game/MyLogic/BPI_Points.Peredacha` Points) 3)
    (`|SpawnActorFromClass` "/Game/MyLogic/BP_Spawner.BP_Spawner_C" (`KismetMathLibrary.MakeTransform` (`SceneComponent.K2_GetComponentLocation` (`self.Cube`))) "Undefined" "OverrideRootScale" null null))
  (`ActorComponent.K2_DestroyComponent` (`self.Cube`))
  (bind _outactors (`GameplayStatics.GetAllActorsWithTag` "Setka"))
  (message `/Game/MyLogic/BPI_EndGame.CountOfBlocks` _outactors true)
  (message `/Game/MyLogic/BPI_Points.Nachislenie` _outactors (`self.sc0re`)))

(fn `UserConstructionScript`)