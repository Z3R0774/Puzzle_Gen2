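; BP_Ball is a bouncing ball actor that works with Platform and DZ tagged actors.
; Tick sweeps the sphere along its direction at the current speed and reflects it off the surface normal on blocking hits.
; Events handle launch, repositioning and retagging, and Alive? updates the life flag and messages Platform actors.
; When that flag is false, Tick notifies DZ actors for the ball count and destroys the ball.
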(event `/Game/MyLogic/BPI_KI11.Firestarter`
  (params (NewParam :type Name))
  (set `self.Speed` 2000.0))

(event `/Game/MyLogic/BPI_KI11.Location`
  (params (Location :type "Vector Structure"))
  (`SceneComponent.K2_SetWorldLocation` (`self.Sphere`) Location false false))

(event `/Game/MyLogic/BPI_KI11.Again?`
  (params (`Start?` :type Boolean))
  ;[1 1 1] New start
  (if `Start?`
    (set `self.Speed` 2000.0)
    (set `self.Tags` (`self.ReadyToDie`))))

(event `/Game/MyLogic/BPI_KI11.AnotherOne`
  (params (Name :type Name))
  (set `self.Tags` (`|MakeArray` Name)))

(event `self.ReceiveBeginPlay`
  ;[1 1 1] Begin
  (set `self.LiFeStat` true)
  (set `self.Speed` 0.0))

(event `/Game/MyLogic/BPI_KI11.Alive?`
  (params (LiFeStat :type Boolean))
  ;[1 1 1] Respawn
  (set `self.LiFeStat` LiFeStat)
  (set `self.Tags` (`self.New_0`))
  (bind _output_get (set `self.New Life` true))
  (bind _outactors (`GameplayStatics.GetAllActorsWithTag` "Platform"))
  (message `/Game/MyLogic/BPI_KI11.New?` _outactors _output_get))

(event `self.ReceiveTick`
  (params (DeltaSeconds :type "Float (single-precision)"))
  ;[1 1 1] Movement
  (if (`self.LiFeStat`)
    (bind _sweephitresult (`SceneComponent.K2_AddWorldOffset` (`self.Sphere`) (* (* (`self.Drection`) (`self.Speed`)) DeltaSeconds) true false))
    (bind (_bblockinghit _binitialoverlap _time _distance _location _impactpoint _normal) (`GameplayStatics.BreakHitResult` _sweephitresult))
    (if _bblockinghit
      (set `self.Drection` (`KismetMathLibrary.GetReflectionVector` (`self.Drection`) _normal)))
    (else
      (bind _outactors (`GameplayStatics.GetAllActorsWithTag` "DZ"))
      (message `/Game/MyLogic/BPI_KI11.BallCount` _outactors true)
      (`self.K2_DestroyActor`))))

(fn `UserConstructionScript`)